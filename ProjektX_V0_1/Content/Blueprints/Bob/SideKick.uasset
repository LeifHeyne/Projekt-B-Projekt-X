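; SideKick is a companion that follows the first player's character along the X and Z axes, ignoring Y.
; Each tick it measures the absolute X distance to the player.
; At 300 units or more, it adds movement input along the normalized direction to the player, offset slightly in X, with input scale proportional to that distance.
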(event `CalculateDistance`
  (bind _returnvalue_x (`KismetMathLibrary.BreakVector` (`self.K2_GetActorLocation`)))
  (bind _returnvalue_x_2 (`KismetMathLibrary.BreakVector` (`self.K2_GetActorLocation` (`GameplayStatics.GetPlayerCharacter` 0))))
  (bind _returnvalue (- _returnvalue_x _returnvalue_x_2))
  (if (>= _returnvalue 0.0)
    (set `self.Distance` _returnvalue)
    (else
      (set `self.Distance` (* -1 _returnvalue)))))

(event `self.ReceiveTick`
  (params (DeltaSeconds :type "Float (single-precision)"))
  (bind (_returnvalue_x _returnvalue_y _returnvalue_z) (`KismetMathLibrary.BreakVector` (- (`self.K2_GetActorLocation` (`GameplayStatics.GetPlayerCharacter` 0)) (`self.K2_GetActorLocation`))))
  (bind (_returnvalue_x_2 _returnvalue_y_2 _returnvalue_z_2) (`KismetMathLibrary.BreakVector` (`KismetMathLibrary.Normal` (`KismetMathLibrary.MakeVector` (- _returnvalue_x 50.0) 0.0 _returnvalue_z))))
  (`self.CalculateDistance`)
  (if (>= (`self.Distance`) 300.0)
    (`self.AddMovementInput` (`KismetMathLibrary.MakeVector` _returnvalue_x_2 0.0 _returnvalue_z_2) (* 3 (* (`self.Distance`) 0.001)))))

(fn `UserConstructionScript`)