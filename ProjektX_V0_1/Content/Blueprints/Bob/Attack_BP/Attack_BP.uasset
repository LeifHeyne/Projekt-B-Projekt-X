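; Attack actor, apparently a moving hitbox, that slides from its spawn location to a target point.
; SetVariable sizes the box, stores damage, converts an offset into the target (X mirrored when not moving right) and inverts the duration into a play rate.
; The move event applies that rate and runs a timeline that lerps the actor's location without sweep.
; Damage is only stored; no overlap logic uses it here.
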(event `self.ReceiveBeginPlay`
  (set `self.setLocation` (`self.K2_GetActorLocation`)))

(event `move`
  (`TimelineComponent.SetPlayRate` (`self.Move_Stuff`) (`self.PlayRateInSec`))
  (bind (_direction _alpha) (`Timeline|Move_Stuff` :!via `PlayFromStart`)
    (:`Update`
      (`self.K2_SetActorLocation` (`KismetMathLibrary.VLerp` (`self.setLocation`) (`self.MoveSpace`) _alpha)))))

(fn `SetVariable`
  (params (Shape :type "Vector Structure") (MoveSpace :type "Vector Structure") (Time :type "Float (double-precision)") (`Is movin right` :type Boolean) (Dmg :type "Float (double-precision)"))
  (bind _setlocation (`self.setLocation`))
  (`BoxComponent.SetBoxExtent` (`self.Box`) Shape true)
  (if `Is movin right`
    (set `self.MoveSpace` (+ _setlocation MoveSpace))
    (else
      (set `self.MoveSpace` (+ _setlocation (`KismetMathLibrary.MakeVector` (* (.x MoveSpace) -1.0) (.y MoveSpace) (.z MoveSpace))))))
  (set `self.PlayRateInSec` (`KismetMathLibrary.MultiplyMultiply_FloatFloat` Time -1.0))
  (set `self.Damage` Dmg))

(fn `UserConstructionScript`)