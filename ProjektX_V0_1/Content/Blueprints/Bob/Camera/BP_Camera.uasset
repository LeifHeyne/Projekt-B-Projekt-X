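; Side-scrolling camera that follows a settable target in the X/Z plane, confined by a set of camera zones.
; Trigger events parse a zone name from the passed string, find that zone actor by display name and rebuild Min/Max from its bounds.
; While following, each tick eases past per-axis margins, clamps using those limits and a half-width from FieldOfView and viewport aspect, then interpolates the camera there.
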(event `self.ReceiveBeginPlay`
  ;[0 1 0.9141] Set Cordinates for min max
  (set `self.CurrentIndex` 0)
  (`self.SetCameraZoneMinMax` (`self.CurrentIndex`)))

(event `self.ReceiveTick`
  (params (DeltaSeconds :type "Float (single-precision)"))
  (if (`self.IsFollowing`)
    (`self.Handle Camera Movement` DeltaSeconds)))

(event `/Game/Blueprints/Bob/Camera/Triggers/BP_CameraZone.OnCameraTrigger`
  (params (Name :type String))
  (bind _currentindex (`self.CurrentIndex`))
  (`self.GetCameraZone` Name)
  (if (`self.DoUpdate`)
    (`KismetSystemLibrary.PrintString` (`KismetStringLibrary.Conv_IntToString` _currentindex))
    (`self.SetCameraZoneMinMax` _currentindex)))

(event `/Game/Blueprints/Bob/Camera/Triggers/BP_CameraZone.SetCameraTarget`
  (params (NewTarget :type "Actor Object Reference"))
  ;[1 1 1] Set Camera Target
  (set `self.CameraTarget` NewTarget))

(fn `GetCameraZone`
  (params (Name :type String))
  (bind _returnvalue (`KismetStringLibrary.GetSubstring` Name 1 (- (`KismetStringLibrary.Len` Name) 1)))
  (bind (_lefts _rights _returnvalue_2) (`KismetStringLibrary.Split` _returnvalue "-"))
  ;[1 1 1] Comment
  (if _returnvalue_2
    (set `self.CameraZoneName` _lefts)
    (else
      (set `self.CameraZoneName` _returnvalue)))
  (for (_array_element _array_index) (`self.CameraZone`)
    (if (`KismetStringLibrary.EqualEqual_StrStr` (`KismetSystemLibrary.GetDisplayName` _array_element) (`self.CameraZoneName`))
      (if (!= (`self.CurrentIndex`) _array_index)
        (set `self.CurrentIndex` _array_index)
        (set `self.DoUpdate` true)
        (break)
        (else
          (set `self.DoUpdate` false)
          (break))))))

(fn `Handle Camera Movement`
  (params (DeltaTime :type "Float (double-precision)"))
  (bind _camerahalfwidth (`self.CameraHalfWidth`))
  (bind _camerahalfwidth_2 (`self.CameraHalfWidth`))
  (bind (_sizex _sizey) (`PlayerController.GetViewportSize` (`GameplayStatics.GetPlayerController` 0)))
  ;[1 0.9839 0] Comment
  (set `self.DeltaTime` DeltaTime)
  (set `self.CameraPosX` (.x (`SceneComponent.K2_GetComponentLocation` (`self.CameraComponent`))))
  (set `self.CameraPosZ` (.z (`SceneComponent.K2_GetComponentLocation` (`self.CameraComponent`))))
  ;[1 1 1] Comment
  (if (> (`KismetMathLibrary.Abs` (- (`self.CameraPosX`) (.x (`self.K2_GetActorLocation` (`self.CameraTarget`))))) (`KismetMathLibrary.BreakVector2D` (`self.Margin`)))
    (set `self.CameraPosX` (`KismetMathLibrary.Lerp` (`self.CameraPosX`) (.x (`self.K2_GetActorLocation` (`self.CameraTarget`))) (* (`KismetMathLibrary.BreakVector2D` (`self.Smothing`)) (`local.DeltaTime`)))))
  ;[1 1 1] set Z positioen
  (if (> (`KismetMathLibrary.Abs` (- (`self.CameraPosX`) (.z (`self.K2_GetActorLocation` (`self.CameraTarget`))))) (`.Y` (`KismetMathLibrary.BreakVector2D` (`self.Margin`))))
    (set `self.CameraPosZ` (`KismetMathLibrary.Lerp` (`self.CameraPosZ`) (.z (`self.K2_GetActorLocation` (`self.CameraTarget`))) (* (`.Y` (`KismetMathLibrary.BreakVector2D` (`self.Smothing`))) (`local.DeltaTime`)))))
  ;[1 1 1] Set Half width from field of view
  (set `self.CameraHalfWidth` (* (`self.FieldOfView`) (/ (`KismetMathLibrary.Conv_IntToDouble` _sizex) (`KismetMathLibrary.Conv_IntToDouble` _sizey))))
  ;[0 0.2136 1] Adjust pos x as per camera zone
  (set `self.CameraPosX` (`KismetMathLibrary.FClamp` (`self.CameraPosX`) (+ _camerahalfwidth_2 (.x (`self.Min`))) (- (.x (`self.Max`)) _camerahalfwidth_2)))
  ;[0.7644 0 1] adjust pos z as per camera zone
  (set `self.CameraPosZ` (`KismetMathLibrary.FClamp` (`self.CameraPosZ`) (+ _camerahalfwidth (.x (`self.Min`))) (- (.z (`self.Max`)) _camerahalfwidth)))
  ;[1 0 0.1286] set camera location
  (`SceneComponent.K2_SetWorldLocation` (`self.CameraComponent`) (`KismetMathLibrary.VInterpTo` (`SceneComponent.K2_GetComponentLocation` (`self.CameraComponent`)) (`KismetMathLibrary.MakeVector` (`self.CameraPosX`) (.y (`SceneComponent.K2_GetComponentLocation` (`self.CameraComponent`))) (`self.CameraPosZ`)) (`local.DeltaTime`) 2.0) false false)
  (return))

(fn `SetCameraZoneMinMax`
  (params (Index :type Integer))
  (bind _y (.y (`SceneComponent.K2_GetComponentLocation` (`self.CameraComponent`))))
  (bind (_origin _boxextent) (`self.GetActorBounds` (`|GetArrayItem` (`self.CameraZone`) Index) false))
  ;[0 0.4249 1] Get Bounds: Location(Origins) && HalfLocation (Box Extends)
  (set `self.Location` _origin)
  (set `self.Coordinates` _boxextent)
  ;[1 0.5227 0.1194] Left and Bottom Cooordinat
  (set `self.Min` (`KismetMathLibrary.MakeVector` (- (.x (`self.Location`)) (.x (`self.Coordinates`))) _y (- (.z (`self.Location`)) (.z (`self.Coordinates`)))))
  ;[1 0.8238 0.07005] Top and Right Coordinate
  (set `self.Max` (`KismetMathLibrary.MakeVector` (+ (.x (`self.Location`)) (.x (`self.Coordinates`))) _y (+ (.z (`self.Location`)) (.z (`self.Coordinates`)))))
  (return))

(fn `UserConstructionScript`)