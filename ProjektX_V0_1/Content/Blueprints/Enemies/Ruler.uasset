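; Ruler enemy Blueprint with a simple Idle, Patrolling and Attacking state manager, with no movement logic yet.
; PawnSensing sets InRange on hearing noise and Attacking on seeing a pawn; neither returns to false once true.
; Tick derives the state enum from those flags, writes them back per state, then fires a cooldown-gated attack while Attacking is set.
; The attack itself is a placeholder debug print.
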(event `self.ReceiveTick`
  (params (DeltaSeconds :type "Float (single-precision)"))
  ;[1 0.5359 0.6058] Statemanager
  (`|ExecutionSequence`
    (:`then_1`
      ;;[0.4333 0.6597 1] Status Enum ändern
      (if (`self.InRange`)
        (if (`self.Attacking`)
          (set `self.EnemyStateEnum` "NewEnumerator3")
          (else
            (set `self.EnemyStateEnum` "NewEnumerator1")))
        (else
          (set `self.EnemyStateEnum` "NewEnumerator0"))))
    (:`then_2`
      ;;[0.4333 0.6597 1] Edit Bools je nach Status
      (switch `/Game/Blueprints/Enemies/EnemyState` (`self.EnemyStateEnum`)
        (:`NewEnumerator0`
          (set `self.InRange` false))
        (:`NewEnumerator1`
          (set `self.InRange` true))
        (:`NewEnumerator3`
          (set `self.Attacking` true))))
    (:`then_3`
      ;;[0.4333 0.6597 1] Angriff
      (if (and (`self.CanAttack`) (`self.Attacking`))
        (set `self.CanAttack` false)
        (`self.SummonAttack`)
        (`KismetSystemLibrary.Delay` (`self.Cooldown`))
        (set `self.CanAttack` true)))))

(event `SummonAttack`
  ;[1 0.5359 0.6058] Grundfunktionen
  ;;[0.5875 1 0.6906] Attack
  (`KismetSystemLibrary.PrintString` "Bam stirb!"))

(event `self.PawnSensing.OnHearNoise`
  (params (Instigator :type "Pawn Object Reference") (Location :type "Vector Structure (by ref)") (Volume :type "Float (single-precision)"))
  ;[1 0.5359 0.6058] Grundfunktionen
  ;;[0.6655 1 0.6641] Aktivierung
  (set `self.InRange` true))

(event `self.PawnSensing.OnSeePawn`
  (params (Pawn :type "Pawn Object Reference"))
  ;[1 0.5359 0.6058] Grundfunktionen
  ;;[0.6655 1 0.6641] Angriff starten
  (set `self.Attacking` true))

(fn `UserConstructionScript`)