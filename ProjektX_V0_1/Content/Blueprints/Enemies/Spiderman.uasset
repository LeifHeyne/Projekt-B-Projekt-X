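; Spiderman enemy that throws Bomber_Shoot projectiles at the player when they come within range.
; Each tick it updates the distance and switches its state enum to attack when the player is close and at similar height.
; Attack plays a throw sound, spawns the projectile on the facing side, then holds a five-second cooldown flag.
; While that flag is set, it turns to face the player along the X axis.
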(event `self.ReceiveTick`
  (params (DeltaSeconds :type "Float (single-precision)"))
  (bind _returnvalue_x (`KismetMathLibrary.BreakVector` (`self.K2_GetActorLocation`)))
  (bind (_returnvalue_x_2 _returnvalue_y _returnvalue_z) (`KismetMathLibrary.BreakVector` (`self.K2_GetActorLocation`)))
  (bind (_returnvalue_x_3 _returnvalue_y_2 _returnvalue_z_2) (`KismetMathLibrary.BreakVector` (`self.K2_GetActorLocation`)))
  (bind (_returnvalue_x_4 _returnvalue_y_3 _returnvalue_z_3) (`KismetMathLibrary.BreakVector` (`self.K2_GetActorLocation` (`GameplayStatics.GetPlayerCharacter` 0))))
  (bind _returnvalue_x_5 (`KismetMathLibrary.BreakVector` (`self.K2_GetActorLocation` (`GameplayStatics.GetPlayerCharacter` 0))))
  (bind (_returnvalue_x_6 _returnvalue_y_4 _returnvalue_z_4) (`KismetMathLibrary.BreakVector` (`self.K2_GetActorLocation` (`GameplayStatics.GetPlayerCharacter` 0))))
  (`|ExecutionSequence`
    (:`then_0`
      ;[0.6565 1 0.555] 1. Distanzberechnung
      (`self.CalculateDistance`))
    (:`then_1`
      ;[0.4479 0.5155 1] 2. Setze Enum auf aktuellen Status
      (if (and (<= (`self.Distance`) 900.0) (>= _returnvalue_z_3 (- _returnvalue_z_2 250.0)) (<= _returnvalue_z_4 (+ _returnvalue_z 250.0)))
        (set `self.EnemyStateEnum` "NewEnumerator3")
        (else
          (set `self.EnemyStateEnum` "NewEnumerator0"))))
    (:`then_2`
      ;[0.4479 0.5155 1] 3. Aktion je nach Enum Status
      (if (`|EnumEquality` (`self.EnemyStateEnum`) "NewEnumerator3")
        (`self.Attack`)))
    (:`then_3`
      (if (`self.Attacking`)
        (if (>= _returnvalue_x_5 _returnvalue_x)
          (set `self.IsMovingRight ` true)
          (else
            (set `self.IsMovingRight ` false)))
        (`self.TurnAround`)))))

(event `Attack`
  (bind _returnvalue (`SceneComponent.K2_GetComponentToWorld` (`self.CapsuleComponent`)))
  ;[1 0.6146 0.6146] Attack
  (if (not (`self.Attacking`))
    (set `self.Attacking` true)
    (`GameplayStatics.SpawnSoundAttached` "/Game/Sounds/Enemies/Spider/149802_orginaljun_1-super-fast-throwing-sound__online-audio-converter_com_.149802_orginaljun_1-super-fast-throwing-sound__online-audio-converter_com_" (`self.CapsuleComponent`))
    (if (`self.IsMovingRight `)
      (`|SpawnActorFromClass` "/Game/Blueprints/Enemies/Bomber/Bomber_Shoot.Bomber_Shoot_C" (`KismetMathLibrary.MakeTransform` (`KismetMathLibrary.MakeVector` (+ (.x (.location _returnvalue)) 60.0) (.y (.location _returnvalue)) (.z (.location _returnvalue))) (.rotation _returnvalue)) "AdjustIfPossibleButAlwaysSpawn" "OverrideRootScale" null null)
      (else
        (`|SpawnActorFromClass` "/Game/Blueprints/Enemies/Bomber/Bomber_Shoot.Bomber_Shoot_C" (`KismetMathLibrary.MakeTransform` (`KismetMathLibrary.MakeVector` (- (.x (.location _returnvalue)) 60.0) (.y (.location _returnvalue)) (.z (.location _returnvalue))) (.rotation _returnvalue)) "AdjustIfPossibleButAlwaysSpawn" "OverrideRootScale" null null)))
    (`KismetSystemLibrary.Delay` 5.0)
    (set `self.Attacking` false)))

(fn `UserConstructionScript`
  (`parent.UserConstructionScript`))