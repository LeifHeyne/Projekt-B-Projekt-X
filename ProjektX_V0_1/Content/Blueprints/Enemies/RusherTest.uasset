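; Test version of a Paper2D "Rusher" enemy character that patrols, chases and performs a charge attack.
; Each tick it recalculates distance, derives an enum state from distance and Chasing/Attacking flags, then runs patrol, chase or attack, doing nothing out of range.
; Attack tilts the actor, swaps flipbooks, waits, then launches it horizontally in its movement direction with a slam sound before resuming the chase.
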(event `self.ReceiveTick`
  (params (DeltaSeconds :type "Float (single-precision)"))
  (bind _charactermovement (`self.CharacterMovement`))
  (bind _enemystateenum (`self.EnemyStateEnum`))
  (`|ExecutionSequence`
    (:`then_0`
      ;[0.6565 1 0.555] 1. Distanzberechnung
      (`self.CalculateDistance`))
    (:`then_1`
      ;[0.4479 0.5155 1] 2. Setze Enum auf aktuellen Status
      (if (<= (`self.Distance`) 2000.0)
        (if (`self.Chasing`)
          (if (`self.Attacking`)
            (set `self.EnemyStateEnum` "NewEnumerator3")
            (else
              (set `self.EnemyStateEnum` "NewEnumerator2")))
          (else
            (set `self.EnemyStateEnum` "NewEnumerator1")))
        (else
          (set `self.EnemyStateEnum` "NewEnumerator0"))))
    (:`then_3`
      ;[0.4479 0.5155 1] 3. Aktion je nach Enum Status
      (if (`|EnumEquality` _enemystateenum "NewEnumerator0")
        _
        (elif (`|EnumEquality` _enemystateenum "NewEnumerator1")
          (if (not (`self.Attacking`))
            (`self.Patroll`)
            (set `CharacterMovementComponent.MaxWalkSpeed` 150.0 _charactermovement))
          (elif (`|EnumEquality` _enemystateenum "NewEnumerator2")
            (if (<= (`self.Distance`) 500.0)
              (`self.Attack`)
              (else
                (`self.Chase`)
                (set `CharacterMovementComponent.MaxWalkSpeed` 300.0 _charactermovement)))))))))

(event `Attack`
  ;[1 0.526 0.526] Attack
  (set `self.Chasing` false)
  (set `self.Attacking` true)
  (`self.K2_AddActorLocalRotation` (struct :`Pitch` -45.0))
  (`PaperFlipbookComponent.SetFlipbook` (`self.Sprite`) "/Game/2DSideScroller/Sprites/EnemyTextures/NewEnemies/Rusher_Atta.Rusher_Atta")
  (`KismetSystemLibrary.Delay` 0.5)
  (`GameplayStatics.SpawnSoundAttached` "/Game/Sounds/Enemies/Rusher/NFF-slam.NFF-slam" (`self.CapsuleComponent`) "None" (0.0 0.0 0.0) (struct) "KeepRelativeOffset" false 0.3 2.5)
  (`self.LaunchCharacter` (`KismetMathLibrary.SelectVector` (3000.0 0.0 0.0) (-3000.0 0.0 0.0) (`self.IsMovingRight `)))
  (`KismetSystemLibrary.Delay` 1.0)
  (`self.K2_AddActorLocalRotation` (struct :`Pitch` 45.0))
  (`PaperFlipbookComponent.SetFlipbook` (`self.Sprite`) "/Game/2DSideScroller/Sprites/EnemyTextures/NewEnemies/Rusher_Ani.Rusher_Ani")
  (set `self.Attacking` false)
  (set `self.Chasing` true))

(fn `UserConstructionScript`
  (`parent.UserConstructionScript`))