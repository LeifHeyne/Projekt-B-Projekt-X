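; Batman is an enemy Blueprint that runs a simple Tick-driven state machine for patrolling and chasing.
; Each frame it calls CalculateDistance, then derives EnemyStateEnum from Distance and the Chasing and Attacking flags.
; The state triggers Patroll or Chase, with chasing skipped at close range; the out-of-range and attacking states trigger no action here.
; CalculateDistance, Patroll, Chase and the code setting both flags are defined outside this graph.
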(event `self.ReceiveTick`
  (params (DeltaSeconds :type "Float (single-precision)"))
  (bind _enemystateenum (`self.EnemyStateEnum`))
  (`|ExecutionSequence`
    (:`then_0`
      ;[0.6565 1 0.555] 1. Distanzberechnung
      (`self.CalculateDistance`))
    (:`then_1`
      ;[0.4479 0.5155 1] 2. Setze Enum auf aktuellen Status
      (if (<= (`self.Distance`) 2000.0)
        (if (`self.Chasing`)
          (if (`self.Attacking`)
            (set `self.EnemyStateEnum` "NewEnumerator3")
            (else
              (set `self.EnemyStateEnum` "NewEnumerator2")))
          (else
            (set `self.EnemyStateEnum` "NewEnumerator1")))
        (else
          (set `self.EnemyStateEnum` "NewEnumerator0"))))
    (:`then_3`
      ;[0.4479 0.5155 1] 3. Aktion je nach Enum Status
      (if (`|EnumEquality` _enemystateenum "NewEnumerator0")
        _
        (elif (`|EnumEquality` _enemystateenum "NewEnumerator1")
          (if (not (`self.Attacking`))
            (`self.Patroll`))
          (elif (`|EnumEquality` _enemystateenum "NewEnumerator2")
            (if (not (<= (`self.Distance`) 100.0))
              (`self.Chase`))))))))

(fn `UserConstructionScript`
  (`parent.UserConstructionScript`))